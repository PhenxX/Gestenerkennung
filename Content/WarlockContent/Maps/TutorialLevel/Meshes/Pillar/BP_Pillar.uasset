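; Tutorial-level pillar meant to show a spell tutorial effect at a stone display, but its event logic is currently disconnected.
; Capsule overlap events are empty, and the orphaned input toggles and spawn chain never run.
; That chain uses FindNearestStoneDisplay, a distance search starting at a 5000-unit threshold, then checks IsClear.
; SpellNumber then selects which of the display's eight particle templates to spawn, yaw-offset by 90 degrees.
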(event `self.Capsule.OnComponentBeginOverlap`
  (params (OverlappedComponent :type "PrimitiveComponent Object Reference") (OtherActor :type "Actor Object Reference") (OtherComp :type "PrimitiveComponent Object Reference") (OtherBodyIndex :type Integer) (bFromSweep :type Boolean) (SweepResult :type "HitResult Structure (by ref)")))

(event `self.Capsule.OnComponentEndOverlap`
  (params (OverlappedComponent :type "PrimitiveComponent Object Reference") (OtherActor :type "Actor Object Reference") (OtherComp :type "PrimitiveComponent Object Reference") (OtherBodyIndex :type Integer)))

(event `Key|MotionController_Left_Trigger`
  (params (Key :type "Key Structure")))

(event `Key|MotionController_Right_Trigger`
  (params (Key :type "Key Structure")))

(fn `findNearestStoneDisplay`
  (params (StoneDisplays :type "Array of /Game/WarlockContent/Maps/TutorialLevel/Meshes/StoneDisplay/BP_StoneDisplay Object Reference"))
  (returns (nearestStoneDisplay :type "/Game/WarlockContent/Maps/TutorialLevel/Meshes/StoneDisplay/BP_StoneDisplay Object Reference"))
  (set `self.smallestStoneDPdistance` 5000.0)
  (for (_array_element _array_index) StoneDisplays
    (bind _returnvalue (`KismetMathLibrary.Abs` (`self.GetDistanceTo` _array_element)))
    (if (< _returnvalue (`self.smallestStoneDPdistance`))
      (set `self.smallestStoneDPdistance` _returnvalue)
      (set `self.indexStoneDisplay` _array_index)))
  (return (`|GetArrayItem` StoneDisplays (`self.indexStoneDisplay`))))

(fn `UserConstructionScript`)