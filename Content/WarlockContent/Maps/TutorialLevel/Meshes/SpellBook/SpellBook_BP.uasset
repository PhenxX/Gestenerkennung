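; SpellBook_BP is a spell book prop in the tutorial level that floats up and down in place.
; BeginPlay starts a fast looping timer on the "float" function, which nudges the actor vertically by a scaled cosine of X instead of using Tick.
; X ping-pongs between -1 and 1, starting from a random value set in the construction script to vary the phase.
; The stored initial location is never read.
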(event `self.ReceiveBeginPlay`
  (`KismetSystemLibrary.K2_SetTimer` self "float" 0.04 true))

(fn `float`
  (bind _returnvalue (+ (`self.x`) (`self.step`)))
  (`self.K2_AddActorWorldOffset` (`KismetMathLibrary.MakeVector` 0.0 0.0 (* (`KismetMathLibrary.Cos` (`KismetMathLibrary.MultiplyByPi` (`self.x`))) 0.05)))
  (if (>= _returnvalue 1.0)
    (set `self.step` -0.01)
    (elif (<= _returnvalue -1.0)
      (set `self.step` 0.01)
      (else
        (set `self.x` _returnvalue))))
  (return))

(fn `UserConstructionScript`
  (set `self.initLocation` (`SceneComponent.K2_GetComponentLocation` (`self.StaticMeshComponent`)))
  (set `self.x` (`KismetMathLibrary.RandomFloatInRange` -1.0 1.0))
  (set `self.step` 0.01))