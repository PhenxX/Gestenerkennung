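; VR explosion spell that follows the owner's motion controller and detonates where it is aimed.
; Once confirmed, Tick line-traces forward from the controller, showing a beam only while it hits a Cube_Blueprint.
; With the beam visible, trigger press re-traces and spawns an explosion effect at the hit.
; It fakes the blast physics with a briefly spawned invisible, heavy, oversized Cube_Blueprint, then calls Kill.
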(event `self.ReceiveTick`
  (params (DeltaSeconds :type "Float (single-precision)"))
  (bind _particlesystem (`self.ParticleSystem`))
  (bind _returnvalue (`self.GetComponentByClass` (`self.GetOwner`) "/Script/HeadMountedDisplay.MotionControllerComponent"))
  (bind _returnvalue_2 (`SceneComponent.K2_GetComponentLocation` _returnvalue))
  ;[1 1 1] Tick: relocate Sphere to be on casting hand
  (`SceneComponent.K2_SetWorldTransform` (`self.Sphere`) (`SceneComponent.K2_GetComponentToWorld` _returnvalue) false false)
  (if (`self.isActivated`)
    (bind _outhit (`KismetSystemLibrary.LineTraceSingle` :`Start` _returnvalue_2 :`End` (+ _returnvalue_2 (* (`SceneComponent.GetForwardVector` _returnvalue) 5000.0)) :`TraceChannel` "TraceTypeQuery1" :`DrawTime` 1.0))
    (bind (_bblockinghit _binitialoverlap _time _location _impactpoint _normal _impactnormal _physmat _hitactor) (`GameplayStatics.BreakHitResult` _outhit))
    (cast `/Game/WarlockContent/Maps/TutorialLevel/Meshes/Cube_Blueprint` _hitactor
      (:`then`
        (`SceneComponent.SetVisibility` _particlesystem true false)
        (`ParticleSystemComponent.SetBeamSourcePoint` _particlesystem 0 (`SceneComponent.K2_GetComponentLocation` (`self.GetComponentByClass` (`self.GetOwner`) "/Script/HeadMountedDisplay.MotionControllerComponent")) 0)
        (`ParticleSystemComponent.SetBeamTargetPoint` _particlesystem 0 _location 0))
      (:`CastFailed`
        (`SceneComponent.SetVisibility` _particlesystem false false)))))

(event `/Game/WarlockContent/MagicBlueprints/MagicInterface.triggerPressed`
  (bind _returnvalue (`self.GetComponentByClass` (`self.GetOwner`) "/Script/HeadMountedDisplay.MotionControllerComponent"))
  (bind _returnvalue_2 (`SceneComponent.K2_GetComponentLocation` _returnvalue))
  ;[1 1 1] OnTrigger activate Explosion
  (if (`SceneComponent.IsVisible` (`self.ParticleSystem`))
    (bind _outhit (`KismetSystemLibrary.LineTraceSingle` :`Start` _returnvalue_2 :`End` (+ _returnvalue_2 (* (`SceneComponent.GetForwardVector` _returnvalue) 5000.0)) :`TraceChannel` "TraceTypeQuery1" :`DrawTime` 1.0))
    (bind (_bblockinghit _binitialoverlap _time _location) (`GameplayStatics.BreakHitResult` _outhit))
    (`GameplayStatics.SpawnEmitterAtLocation` "/Game/WarlockContent/MagicBlueprints/Explosion/P_Explosion.P_Explosion" _location)
    (`KismetSystemLibrary.Delay` 0.5)
    (bind _returnvalue_3 (`|SpawnActorFromClass` "/Game/WarlockContent/Maps/TutorialLevel/Meshes/Cube_Blueprint.Cube_Blueprint_C" (`KismetMathLibrary.MakeTransform` _location (struct) (2.0 2.0 2.0)) "Undefined" "OverrideRootScale" self))
    (bind _staticmeshcomponent (`StaticMeshActor.StaticMeshComponent` _returnvalue_3))
    (`PrimitiveComponent.SetMassOverrideInKg` _staticmeshcomponent "None" 1000.0 true)
    (`PrimitiveComponent.SetSimulatePhysics` _staticmeshcomponent true)
    (`SceneComponent.SetVisibility` _staticmeshcomponent false false)
    (`KismetSystemLibrary.Delay` 0.5)
    (`self.K2_DestroyActor` _returnvalue_3)
    (`self.kill`)))

(event `/Game/WarlockContent/MagicBlueprints/MagicInterface.confirm`
  (`parent.confirm`)
  (set `self.isActivated` true))

(fn `UserConstructionScript`)