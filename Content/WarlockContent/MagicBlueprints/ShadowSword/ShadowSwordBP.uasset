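; Shadow sword spell Blueprint that puts a sword in place of the owning VR hand while the trigger is held.
; Each tick it moves its root, with sweep, to the owner's motion controller transform.
; Trigger press hides the owner's skeletal mesh, shows the sword and makes it block a custom collision channel.
; Trigger release shows that mesh again and calls Kill on the spell.
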(event `self.ReceiveTick`
  (params (DeltaSeconds :type "Float (single-precision)"))
  (`SceneComponent.K2_SetWorldTransform` (`self.DefaultSceneRoot`) (`SceneComponent.K2_GetComponentToWorld` (`self.GetComponentByClass` (`self.GetOwner`) "/Script/HeadMountedDisplay.MotionControllerComponent")) true false))

(event `/Game/WarlockContent/MagicBlueprints/MagicInterface.triggerPressed`
  (`SceneComponent.SetVisibility` (`self.GetComponentByClass` (`self.GetOwner`) "/Script/Engine.SkeletalMeshComponent") false false)
  (`SceneComponent.SetVisibility` (`self.Sword`) true false)
  (`PrimitiveComponent.SetCollisionResponseToChannel` (`self.Sword`) "ECC_GameTraceChannel5" "ECR_Block"))

(event `/Game/WarlockContent/MagicBlueprints/MagicInterface.triggerReleased`
  (`SceneComponent.SetVisibility` (`self.GetComponentByClass` (`self.GetOwner`) "/Script/Engine.SkeletalMeshComponent") true false)
  (`/Game/WarlockContent/MagicBlueprints/MagicInterface.kill`))

(fn `UserConstructionScript`
  (`parent.UserConstructionScript`))