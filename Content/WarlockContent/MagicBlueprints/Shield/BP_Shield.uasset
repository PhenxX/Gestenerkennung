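; BP_Shield is a VR shield spell actor, owned by a motion controller, that appears while the trigger is held.
; Each tick it snaps its root to the controller's location, keeping only yaw so it stays upright, with the left hand's yaw flipped 180 degrees.
; Trigger press makes the Shield component visible, and release calls Kill.
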(event `self.ReceiveTick`
  (params (DeltaSeconds :type "Float (single-precision)"))
  (bind _location (.location (`SceneComponent.K2_GetComponentToWorld` (`self.GetComponentByClass` (`self.GetOwner`) "/Script/HeadMountedDisplay.MotionControllerComponent"))))
  (bind _yaw (.yaw (.rotation (`SceneComponent.K2_GetComponentToWorld` (`self.GetComponentByClass` (`self.GetOwner`) "/Script/HeadMountedDisplay.MotionControllerComponent")))))
  (bind _asvr_motion_controller (cast `/Game/WarlockContent/VR-Blueprints/VR_MotionController` (`self.GetOwner`)))
  (switch `EControllerHand` (`/Game/WarlockContent/VR-Blueprints/VR_MotionController.Hand` _asvr_motion_controller)
    (:`Left`
      (`SceneComponent.K2_SetWorldTransform` (`self.DefaultSceneRoot`) (`KismetMathLibrary.MakeTransform` _location (`KismetMathLibrary.MakeRotator` 0.0 0.0 (+ _yaw 180.0))) false false))
    (:`Right`
      (`SceneComponent.K2_SetWorldTransform` (`self.DefaultSceneRoot`) (`KismetMathLibrary.MakeTransform` _location (`KismetMathLibrary.MakeRotator` 0.0 0.0 _yaw)) false false))))

(event `/Game/WarlockContent/MagicBlueprints/MagicInterface.triggerPressed`
  (`SceneComponent.SetVisibility` (`self.Shield`) true false))

(event `/Game/WarlockContent/MagicBlueprints/MagicInterface.triggerReleased`
  (`/Game/WarlockContent/MagicBlueprints/MagicInterface.kill`))

(fn `UserConstructionScript`
  (`parent.UserConstructionScript`))