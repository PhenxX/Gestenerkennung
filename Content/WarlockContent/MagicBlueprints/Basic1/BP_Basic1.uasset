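; BP_Basic1 is a basic VR spell actor that appears and propels itself by physics once confirmed.
; Confirm checks that its owner is a VR_MotionController owned by a VR_Pawn, then shows the Basic1 component and activates PhysicsThruster.
; An unconnected draft would orient Basic1 from the camera position and the controller's begin and end cast locations, but it never runs.
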(event `/Game/WarlockContent/MagicBlueprints/MagicInterface.confirm`
  (bind _asvr_motion_controller (cast `/Game/WarlockContent/VR-Blueprints/VR_MotionController` (`self.GetOwner`)))
  (bind _asvr_pawn (cast `/Game/WarlockContent/VR-Blueprints/VR_Pawn` (`self.GetOwner` _asvr_motion_controller)))
  (`SceneComponent.SetVisibility` (`self.Basic1`) true false)
  (`ActorComponent.SetActive` (`self.PhysicsThruster`) true false))

(fn `UserConstructionScript`
  (`parent.UserConstructionScript`))