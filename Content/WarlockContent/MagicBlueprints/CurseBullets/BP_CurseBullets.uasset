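; BP_CurseBullets is a hand-held spell that fires up to ten BP_CurseBullets_Shot projectiles from its owner's motion controller.
; It follows the controller every tick and spawns a shot at that transform on each trigger press.
; Confirm hides the owner's skeletal mesh.
; Kill restores the mesh and calls the parent Kill, after the tenth shot or when the Sphere component registers a hit.
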(event `self.ReceiveTick`
  (params (DeltaSeconds :type "Float (single-precision)"))
  ;[1 1 1] Tick: relocate Sphere to be on casting hand
  (`SceneComponent.K2_SetWorldTransform` (`self.DefaultSceneRoot`) (`SceneComponent.K2_GetComponentToWorld` (`self.GetComponentByClass` (`self.GetOwner`) "/Script/HeadMountedDisplay.MotionControllerComponent")) false false))

(event `/Game/WarlockContent/MagicBlueprints/MagicInterface.triggerPressed`
  ;[1 1 1] OnTrigger activate Thruster
  (`|SpawnActorFromClass` "/Game/WarlockContent/MagicBlueprints/CurseBullets/BP_CurseBullets_Shot.BP_CurseBullets_Shot_C" (`SceneComponent.K2_GetComponentToWorld` (`self.GetComponentByClass` (`self.GetOwner`) "/Script/HeadMountedDisplay.MotionControllerComponent")) "Undefined" "OverrideRootScale" self)
  (bind _output_get (set `self.shotsFired` (+ (`self.shotsFired`) 1)))
  (if (not (< _output_get 10))
    (`self.kill`)))

(event `self.Sphere.OnComponentHit`
  (params (HitComponent :type "PrimitiveComponent Object Reference") (OtherActor :type "Actor Object Reference") (OtherComp :type "PrimitiveComponent Object Reference") (NormalImpulse :type "Vector Structure") (Hit :type "HitResult Structure (by ref)"))
  ;[1 1 1] OnHit show Explosion and kill
  (`self.kill`))

(event `/Game/WarlockContent/MagicBlueprints/MagicInterface.confirm`
  ;[1 1 1] set controller invisable
  (`parent.confirm`)
  (`SceneComponent.SetVisibility` (`self.GetComponentByClass` (`self.GetOwner`) "/Script/Engine.SkeletalMeshComponent") false false))

(event `/Game/WarlockContent/MagicBlueprints/MagicInterface.kill`
  (`SceneComponent.SetVisibility` (`self.GetComponentByClass` (`self.GetOwner`) "/Script/Engine.SkeletalMeshComponent") true false)
  (`parent.kill`))

(fn `UserConstructionScript`)